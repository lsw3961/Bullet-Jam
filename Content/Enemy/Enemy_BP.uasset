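; Enemy actor that turns to face the player, fires projectiles, and opens the VictoryScreen level when its health runs out.
; Tick rotates it toward the player every frame.
; PawnSensing sightings of the player call Attack, which spawns a projectile immediately and sets a looping timer back to Attack.
; Projectiles spawn at the ProjectileSpawn transform, while the delayed code aiming their velocity at the player is disconnected.
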(event OnSeePawn(PawnSensing)
  (params (Pawn :type Pawn%20Object%20Reference))
  (Utilities|Casting|CastToBP_FirstPersonCharacter Pawn)
  (CallFunction|Attack))

(event Custom|Spawn%20Projectile
  (bind _returnvalue (Game|SpawnActorfromClass "/Game/Enemy/Enemy_Projectile_BP.Enemy_Projectile_BP_C" (Transformation|GetWorldTransform (Variables|Default|GetProjectile%20Spawn)) "Undefined" 0 0.0 0)))

(event Custom|Face%20Player
  (Transformation|SetActorRotation (Math|Rotator|FindLookatRotation (Transformation|GetActorLocation) (Transformation|GetActorLocation (Game|GetPlayerCharacter 0)))))

(event Custom|Attack
  (Utilities|Time|SetTimerbyEvent (delegate Custom|Attack) 2.0 true)
  (CallFunction|SpawnProjectile))

(event EventTick
  (params (DeltaSeconds :type Float%20%28single-precision%29))
  (CallFunction|FacePlayer))

(event EventGetHurt
  (params (Damage :type Float%20%28double-precision%29))
  (bind _output_get (Variables|Default|Sethealth (- (Variables|Default|Gethealth) Damage)))
  (if (<= _output_get 0.0)
    (Game|OpenLevel(byName) "VictoryScreen")))

(fn ConstructionScript)