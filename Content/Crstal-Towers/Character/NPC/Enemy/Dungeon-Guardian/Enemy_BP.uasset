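; Dungeon guardian boss enemy that faces the player and fires projectiles, with a health bar on screen.
; Every tick it yaws toward the player; pawn sensing triggers a delayed attack that repeats on a timer, playing a punch animation before spawning each projectile.
; Damage updates the health bar, and reaching zero health opens the outro level.
; The code aiming projectile velocity at the player is disconnected and never runs.
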(event OnSeePawn(PawnSensing)
  (params (Pawn :type Pawn%20Object%20Reference))
  (Utilities|Casting|CastToBP_FirstPersonCharacter Pawn)
  (Utilities|FlowControl|Delay 2.4)
  (CallFunction|Attack))

(event Custom|Spawn%20Projectile
  (Components|Animation|PlayAnimation (Variables|Default|GetSkeletalMesh) "/Game/Crstal-Towers/Character/NPC/Enemy/Dungeon-Guardian/Enemy_Anim/Enemy_anim_punch_Anim.Enemy_anim_punch_Anim" false)
  (Utilities|FlowControl|Delay 1.5)
  (bind _returnvalue (Game|SpawnActorfromClass "/Game/Crstal-Towers/Character/NPC/Enemy/Dungeon-Guardian/Enemy_Projectile_BP.Enemy_Projectile_BP_C" (Transformation|GetWorldTransform (Variables|Default|GetProjectile%20Spawn)) "Undefined" 0 1e+01 0))
  (Utilities|FlowControl|Delay 0.9))

(event Custom|Face%20Player
  (Transformation|SetActorRotation (Math|Rotator|MakeRotator 0.0 0.0 (.yaw (Math|Rotator|FindLookatRotation (Transformation|GetActorLocation) (Transformation|GetActorLocation (Game|GetPlayerCharacter 0)))))))

(event Custom|Attack
  (Utilities|Time|SetTimerbyEvent (delegate Custom|Attack) 5.0 true)
  (CallFunction|SpawnProjectile))

(event EventBeginPlay
  (bind _returnvalue (UserInterface|CreateWidget "/Game/Crstal-Towers/UI/Widgets/BossHealthBar.BossHealthBar_C"))
  (bind _output_get (Variables|Default|SetBoss%20Health%20bar _returnvalue))
  (UserInterface|Viewport|AddtoViewport _output_get 0))

(event EventTick
  (params (DeltaSeconds :type Float%20%28single-precision%29))
  (CallFunction|FacePlayer))

(event EventGetHurt
  (params (Damage :type Float%20%28double-precision%29))
  (bind _output_get (Variables|Default|Sethealth (- (Variables|Default|Gethealth) Damage)))
  (Default|SetHealth (Variables|Default|GetBoss%20Health%20bar) _output_get)
  (if (<= _output_get 0.0)
    (Game|OpenLevel(byName) "OutroSequence")))

(fn ConstructionScript)