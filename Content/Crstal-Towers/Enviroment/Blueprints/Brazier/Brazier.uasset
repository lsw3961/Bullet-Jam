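; Brazier actor that can be lit by fire and put out by ice, acting as a trigger for another actor.
; DoonFire activates the flame effect, sets the mesh material and sends BrazierActivateMessage to ActorToActivate, passing itself.
; IsIceable calls TurnOff, which deactivates the flame and sets the material on the same slot without notifying the linked actor.
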(event Custom|Turn%20Off
  (Components|Activation|Deactivate (Variables|Default|GetBrazierFlame))
  (Rendering|Material|SetMaterial (Variables|Default|GetSM_Brazier) 0 0))

(event EventIsIceable
  (params (Exit :type Boolean) (NewParam :type Splotch%20Decal%20Object%20Reference))
  (CallFunction|TurnOff))

(event EventDoonFire
  (Components|Activation|Activate (Variables|Default|GetBrazierFlame) false)
  (Rendering|Material|SetMaterial (Variables|Default|GetSM_Brazier) 0 0)
  (Class|BrazierActivate|BrazierActivate(Message) (Variables|Default|GetActor%20To%20Activate) self))

(fn ConstructionScript)