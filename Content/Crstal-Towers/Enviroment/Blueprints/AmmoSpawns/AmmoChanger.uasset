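; AmmoChanger is a crystal ammo pickup that refills one ammo type for the first-person player and regrows after a delay.
; Box overlap by that character adds an interaction widget to the viewport and removes it on exit.
; When regenerated, Activate sets the CurrentKey entry in the character's AmmoQuantities map to MaxAmmo, if present, then hides the crystals.
; A timer calls Regenerate to show them and re-enable pickup.
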(event OnComponentBeginOverlap(Box)
  (params (OverlappedComponent :type Primitive%20Component%20Object%20Reference) (OtherActor :type Actor%20Object%20Reference) (OtherComp :type Primitive%20Component%20Object%20Reference) (OtherBodyIndex :type Integer) (bFromSweep :type Boolean) (SweepResult :type Hit%20Result%20Structure%20%28by%20ref%29))
  (Utilities|Casting|CastToBP_FirstPersonCharacter OtherActor)
  (bind _returnvalue (UserInterface|CreateWidget "/Game/Crstal-Towers/UI/Widgets/Player-HUD/InteractionUI.InteractionUI_C"))
  (bind _output_get (Variables|Default|SetInteractionUI _returnvalue))
  (UserInterface|Viewport|AddtoViewport _output_get 0)
  (Development|PrintString "Added"))

(event OnComponentEndOverlap(Box)
  (params (OverlappedComponent :type Primitive%20Component%20Object%20Reference) (OtherActor :type Actor%20Object%20Reference) (OtherComp :type Primitive%20Component%20Object%20Reference) (OtherBodyIndex :type Integer))
  (bind _interactionui (Variables|Default|GetInteractionUI))
  (Development|PrintString (Utilities|GetDisplayName OtherComp))
  (Utilities|Casting|CastToBP_FirstPersonCharacter OtherActor)
  (Widget|RemovefromParent _interactionui)
  (Development|PrintString (Utilities|GetDisplayName _interactionui)))

(event EventActivate
  (bind _currentkey (Variables|Default|GetCurrentKey))
  (bind _maxammo (Variables|Default|GetMaxAmmo))
  (if (Variables|Default|GetIsRegenerated) ; Make sure crystals have regened
    ;[0.5481 1 0.8044] Add the proper ammo type to the player's inventory
    (bind _asbp_first_person_character (Utilities|Casting|CastToBP_FirstPersonCharacter (Game|GetPlayerCharacter 0)))
    (if (.ReturnValue (Utilities|Map|Find (Variables|/Game/Crstal-Towers/Character/Player/FirstPerson/Blueprints/BP_FirstPersonCharacter.BP_FirstPersonCharacter_C|GetAmmoQuantities _asbp_first_person_character) _currentkey))
      (Utilities|Map|Add (Variables|/Game/Crstal-Towers/Character/Player/FirstPerson/Blueprints/BP_FirstPersonCharacter.BP_FirstPersonCharacter_C|GetAmmoQuantities _asbp_first_person_character) _currentkey _maxammo)
      (Development|PrintString (Utilities|String|Append (Utilities|String|EnumtoString _currentkey) ": " (Utilities|String|ToString(Integer) _maxammo)))
      (Development|SetHiddeninGame (Variables|Default|GetAmmoFull_low_Crystals) true false) ; Hide crystals when activated
      (Variables|Default|SetIsRegenerated false)
      (Utilities|Time|SetTimerbyFunctionName 0 "Regenerate" (Variables|Default|GetRegenerateTime)))))

(fn ConstructionScript)

(fn Regenerate
  ;[1 1 1] Regenerate crystals and allow interaction again
  (Variables|Default|SetIsRegenerated true)
  (Development|SetHiddeninGame (Variables|Default|GetAmmoFull_low_Crystals) false false))