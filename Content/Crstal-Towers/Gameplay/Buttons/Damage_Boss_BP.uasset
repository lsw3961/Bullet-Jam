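; Button actor, named for damaging the boss, that spawns Enemy_Projectile_BP shots at an offset from the referenced Boss.
; A first-person character overlapping the button spawns a large, downward-pitched projectile.
; BrazierActivate spawns a smaller one with the same damage, turns off the given brazier and teleports the player to a hard-coded location.
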(event OnComponentBeginOverlap(Button)
  (params (OverlappedComponent :type Primitive%20Component%20Object%20Reference) (OtherActor :type Actor%20Object%20Reference) (OtherComp :type Primitive%20Component%20Object%20Reference) (OtherBodyIndex :type Integer) (bFromSweep :type Boolean) (SweepResult :type Hit%20Result%20Structure%20%28by%20ref%29))
  (Utilities|Casting|CastToBP_FirstPersonCharacter OtherActor)
  (Game|SpawnActorfromClass "/Game/Crstal-Towers/Character/NPC/Enemy/Dungeon-Guardian/Enemy_Projectile_BP.Enemy_Projectile_BP_C" (Math|Transform|MakeTransform (+ (Transformation|GetActorLocation (Variables|Default|GetBoss)) (Variables|Default|GetOffset)) "-90.000000, 0, 0" "5.000000,5.000000,5.000000") "Undefined" 0 1e+02 0))

(event EventBrazierActivate
  (params (Brazier :type Brazier%20Object%20Reference))
  (Game|SpawnActorfromClass "/Game/Crstal-Towers/Character/NPC/Enemy/Dungeon-Guardian/Enemy_Projectile_BP.Enemy_Projectile_BP_C" (Math|Transform|MakeTransform (+ (Transformation|GetActorLocation (Variables|Default|GetBoss)) (Variables|Default|GetOffset)) "-90.000000, 0, 0" "3.000000,3.000000,3.000000") "Undefined" 0 1e+02 0)
  (Default|TurnOff Brazier)
  (Transformation|SetActorLocation (Game|GetPlayerCharacter 0) "1460.000000,280.000000,168.848007" false true))

(fn ConstructionScript)